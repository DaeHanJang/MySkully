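; BP_StrongGollemCharacter is the strong golem character, with a punch as its primary action and a chargeable slam as its secondary action.
; The primary action plays a random one of three punch montage sections, guarded by a Punch flag that this graph never clears.
; Holding the secondary action starts the slam montage, and releasing it plays the End section and clears the slam flags.
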(event `self.PrimaryAction`
  (if (not (`self.bPunch`))
    (set `self.bPunch` true)
    (switch `int` (`KismetMathLibrary.RandomIntegerInRange` 0 2)
      (:`0`
        (`self.PlayAnimMontage` "/Game/Character/Strong/Animation/AM_Punch.AM_Punch" 1.0 "Punch1"))
      (:`1`
        (`self.PlayAnimMontage` "/Game/Character/Strong/Animation/AM_Punch.AM_Punch" 1.0 "Punch2"))
      (:`2`
        (`self.PlayAnimMontage` "/Game/Character/Strong/Animation/AM_Punch.AM_Punch" 1.0 "Punch3")))))

(event `self.SecondaryAction`
  (if (not (`self.bSlam`))
    (set `self.bSlam` true)
    (`self.PlayAnimMontage` "/Game/Character/Strong/Animation/AM_Slam.AM_Slam" 1.0 "Start")
    (set `self.bChargeSlam` true)))

(event `self.StopSecondaryAction`
  (if (`self.bChargeSlam`)
    (set `self.bChargeSlam` false)
    (`self.PlayAnimMontage` "/Game/Character/Strong/Animation/AM_Slam.AM_Slam" 1.0 "End")
    (set `self.bSlam` false)))

(fn `UserConstructionScript`)